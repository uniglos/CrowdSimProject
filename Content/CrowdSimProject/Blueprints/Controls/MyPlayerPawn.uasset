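; Player pawn for the crowd simulation project, providing camera zoom and a hotkey for spawning AI.
; Holding right mouse sets a narrower target FOV that the mouse wheel adjusts, capped only at the default wide value; release restores the default.
; Tick lerps the camera toward the target by a fixed per-frame alpha, slower while held.
; Pressing F spawns a BT_Ai actor at a hardcoded location and prints a debug message.
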(event EventBeginPlay)

(event Collision|EventActorBeginOverlap
  (params (OtherActor :type Actor%20Object%20Reference)))

(event EventTick
  (params (DeltaSeconds :type Float%20%28single-precision%29))
  (bind _camera (Variables|Default|GetCamera))
  (bind _desiredfov (Variables|Default|GetDesiredFOV))
  (bind _fieldofview (Variables|/Script/Engine.CameraComponent|GetFieldOfView _camera))
  (if (Variables|Default|GetRMB_Flag)
    (Camera|SetFieldOfView _camera (Math|Float|Lerp _fieldofview _desiredfov 0.1))
    (else
      (Camera|SetFieldOfView _camera (Math|Float|Lerp _fieldofview _desiredfov 0.5)))))

(event Input|MouseEvents|MouseWheelAxis
  (params (AxisValue :type Float%20%28single-precision%29))
  (if (Variables|Default|GetRMB_Flag)
    (bind _output_get (Variables|Default|SetDesiredFOV (+ (* AxisValue -4.0) (Variables|Default|GetDesiredFOV))))
    (if (>= _output_get 1e+02)
      (Variables|Default|SetDesiredFOV 1e+02))))

(event Input|MouseEvents|RightMouseButton
  (params (Key :type Key%20Structure :default "None"))
  (:Pressed
    (Variables|Default|SetRMB_Flag true)
    (Variables|Default|SetDesiredFOV 5e+01))
  (:Released
    (Variables|Default|SetRMB_Flag false)
    (Variables|Default|SetDesiredFOV 1e+02)))

(event Input|KeyboardEvents|F
  (params (Key :type Key%20Structure :default "None"))
  (:Pressed
    (Game|SpawnActorfromClass "/Game/CrowdSimProject/Blueprints/AI/BT/BT_Ai.BT_Ai_C" (Math|Transform|MakeTransform "1775.000000,-1855.000000,100.000000") "Undefined" "MultiplyWithRoot" 0 0)
    (Development|PrintString "Hello")))

(fn ConstructionScript)